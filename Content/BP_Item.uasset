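; BP_Item is an item actor that travels horizontally to a random box and then drops under physics.
; On BeginPlay it picks a random "Box"-tagged component from the BP_Boxes actor and disables its own tick.
; When tick is enabled, it sweeps toward that box at its current height by Speed per frame, without delta-time scaling.
; Within 10 units, it turns on physics simulation for its static mesh.
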(event EventBeginPlay
  (bind _returnvalue (Actor|GetActorOfClass "/Game/BP_Boxes.BP_Boxes_C"))
  (Variables|Default|SetBox (.OutItem (Utilities|Array|Random (Actor|GetComponentsbyTag _returnvalue "/Script/Engine.SceneComponent" "Box"))))
  (Actor|Tick|SetActorTickEnabled false))

(event Collision|EventActorBeginOverlap
  (params (OtherActor :type Actor%20Object%20Reference)))

(event EventTick
  (params (DeltaSeconds :type Float%20%28single-precision%29))
  (bind _returnvalue (Transformation|GetActorLocation))
  (bind _box (Variables|Default|GetBox))
  (bind _returnvalue_2 (Transformation|GetWorldLocation _box))
  (bind _returnvalue_3 (- (Math|Vector|MakeVector (.x _returnvalue_2) (.y _returnvalue_2) (.z _returnvalue)) (Math|Vector|MakeVector (.x _returnvalue) (.y _returnvalue) (.z _returnvalue))))
  (if (> (Math|Vector|VectorLength _returnvalue_3) 1e+01)
    (Transformation|SetActorLocation (+ (Transformation|GetActorLocation) (* (Math|Vector|Normalize _returnvalue_3) (Variables|Default|GetSpeed))) true false)
    (else
      (Physics|SetSimulatePhysics (Variables|Default|GetStaticMesh) true))))

(fn ConstructionScript)