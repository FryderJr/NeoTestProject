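; BP_Boxes is an actor that spawns a row of BP_Item actors and lets number keys activate them individually.
; On BeginPlay it spawns ten items spaced along X, passing each its index and storing them in an array.
; A numeric key press converts the key's display name to an array index and enables tick on that item if valid.
; Two box components destroy any BP_Item that overlaps them.
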(event OnComponentBeginOverlap(Box)
  (params (OverlappedComponent :type Primitive%20Component%20Object%20Reference) (OtherActor :type Actor%20Object%20Reference) (OtherComp :type Primitive%20Component%20Object%20Reference) (OtherBodyIndex :type Integer) (bFromSweep :type Boolean) (SweepResult :type Hit%20Result%20Structure%20%28by%20ref%29))
  (bind _asbp_item (Utilities|Casting|CastToBP_Item OtherActor))
  (Actor|DestroyActor _asbp_item))

(event OnComponentBeginOverlap(Box1)
  (params (OverlappedComponent :type Primitive%20Component%20Object%20Reference) (OtherActor :type Actor%20Object%20Reference) (OtherComp :type Primitive%20Component%20Object%20Reference) (OtherBodyIndex :type Integer) (bFromSweep :type Boolean) (SweepResult :type Hit%20Result%20Structure%20%28by%20ref%29))
  (bind _asbp_item (Utilities|Casting|CastToBP_Item OtherActor))
  (Actor|DestroyActor _asbp_item))

(event EventBeginPlay
  (for _index (range 0 9)
    (bind _returnvalue (Game|SpawnActorfromClass "/Game/BP_Item.BP_Item_C" (Math|Transform|MakeTransform (+ (Variables|Default|GetSpawn%20Transform%20Location) (Math|Vector|MakeVector (* _index 1e+02) 0.0 0.0)) "0, 0, 0" "1.000000,1.000000,1.000000") "Undefined" "MultiplyWithRoot" 0 _index 0))
    (Utilities|Array|Add (Variables|Default|GetItems) _returnvalue)))

(event Collision|EventActorBeginOverlap
  (params (OtherActor :type Actor%20Object%20Reference)))

(event EventTick
  (params (DeltaSeconds :type Float%20%28single-precision%29)))

(event Input|KeyboardEvents|AnyKey
  (params (Key :type Key%20Structure :default "None"))
  (bind _returnvalue (Class|KismetInputLibrary|KeyGetDisplayName Key true))
  (bind _items (Variables|Default|GetItems))
  (bind _returnvalue_2 (Utilities|String|ToString(Text) _returnvalue))
  (bind _returnvalue_3 (Math|Conversions|ToInteger(Byte) _returnvalue_2))
  (bind _output (Utilities|Array|Get(acopy) _items _returnvalue_3))
  (:Pressed
    (if (Class|KismetStringLibrary|IsNumeric _returnvalue_2)
      (Utilities|IsValid _output
        (:Is%20Valid
          (Actor|Tick|SetActorTickEnabled _output true))))))

(fn ConstructionScript)